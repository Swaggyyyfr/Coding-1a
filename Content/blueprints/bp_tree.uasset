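; Banana plant tree actor that plays a one-time, randomized scale bounce a few seconds after BeginPlay.
; After a random delay, it enlarges the mesh from its current scale, then shrinks it and settles it near full size in short, instant steps.
; The last two steps randomize each axis independently, so the final proportions vary per instance.
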(event `self.ReceiveBeginPlay`
  (bind _returnvalue (`KismetMathLibrary.RandomFloatInRange` 0.7 0.9))
  (bind _returnvalue_2 (`KismetMathLibrary.RandomFloatInRange` 0.9 1.1))
  (bind _sm_bananaplant (`self.SM_BananaPlant`))
  (`KismetSystemLibrary.Delay` (`KismetMathLibrary.RandomFloatInRange` 4.0 6.0))
  (`SceneComponent.SetRelativeScale3D` _sm_bananaplant (+ (`SceneComponent.RelativeScale3D` _sm_bananaplant) (`KismetMathLibrary.RandomFloatInRange` 0.2 0.4)))
  (`KismetSystemLibrary.Delay` 0.2)
  (`SceneComponent.SetRelativeScale3D` _sm_bananaplant (`KismetMathLibrary.MakeVector` _returnvalue _returnvalue _returnvalue))
  (`KismetSystemLibrary.Delay` 0.2)
  (`SceneComponent.SetRelativeScale3D` _sm_bananaplant (`KismetMathLibrary.MakeVector` _returnvalue_2 _returnvalue_2 _returnvalue_2)))

(fn `UserConstructionScript`)
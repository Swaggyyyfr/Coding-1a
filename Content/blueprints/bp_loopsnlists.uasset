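; Blueprint actor that exercises loops and array lookups on BeginPlay, judging by its name and mechanics.
; A Sequence starts two delayed branches: a while loop prints a countdown, cycling text colors from an array by modulo.
; The other calls MakeCoinsJump, which raises the root component of every Bp_key actor, prints how many moved, then re-calls itself after a delay, so keys keep climbing indefinitely.
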(event `self.ReceiveBeginPlay`
  (bind _while_counter (`self.while counter`))
  (`|ExecutionSequence`
    (:`then_0`
      (`KismetSystemLibrary.Delay` 0.2)
      (while (> _while_counter 0)
        (`KismetSystemLibrary.PrintText` (`|FormatText` "we are in the loop number {count}." _while_counter) true true (`|GetArrayItem` (`self.colors`) (mod (`self.while counter`) 7)))
        (`/Engine/EditorBlueprintResources/StandardMacros.DecrementInt` (`self.while counter`))))
    (:`then_1`
      (`KismetSystemLibrary.Delay` 0.2)
      (`self.make coins jump`))))

(event `make coins jump`
  (bind _outactors (`GameplayStatics.GetAllActorsOfClass` "/Game/blueprints/bp_key.bp_key_C"))
  (for _array_element _outactors
    (`SceneComponent.K2_AddRelativeLocation` (`/Game/blueprints/bp_key.DefaultSceneRoot` _array_element) (0.0 0.0 50.0) false false))
  (`KismetSystemLibrary.PrintText` (`|FormatText` "We have raised {count} keys" (`KismetArrayLibrary.Array_Length` _outactors)))
  (`KismetSystemLibrary.Delay` 1.0)
  (`self.make coins jump`))

(fn `UserConstructionScript`)
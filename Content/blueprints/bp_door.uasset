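; BP_Door is a key-locked door that opens when the third-person character overlaps it.
; On overlap it checks the character's TotalKeys; with at least one key it spends one and plays a timeline that lerps the door mesh upward along Z.
; Without keys it prints a denial message and stays shut, and nothing in the graph closes the door again.
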(event `self.ReceiveActorBeginOverlap`
  (params (OtherActor :type "Actor Object Reference"))
  (bind _asbp_third_person_character (cast `/Game/ThirdPerson/Blueprints/BP_ThirdPersonCharacter` OtherActor))
  (if (> (`/Game/ThirdPerson/Blueprints/BP_ThirdPersonCharacter.TotalKeys` _asbp_third_person_character) 0)
    (`/Engine/EditorBlueprintResources/StandardMacros.DecrementInt` (`/Game/ThirdPerson/Blueprints/BP_ThirdPersonCharacter.TotalKeys` _asbp_third_person_character)
      (:`  `
        (`KismetSystemLibrary.PrintText` "Welcome!")
        (bind (_direction _newtrack_0) (`Timeline|Timeline`)
          (:`Update`
            (`SceneComponent.K2_SetRelativeLocation` (`self.SM_Storage01_Door`) (`KismetMathLibrary.MakeVector` 0.0 0.0 (`KismetMathLibrary.Lerp` 0.0 210.0 _newtrack_0)) false false)))))
    (else
      (`KismetSystemLibrary.PrintText` "DENIED! \nGo do some parkour."))))

(fn `UserConstructionScript`)
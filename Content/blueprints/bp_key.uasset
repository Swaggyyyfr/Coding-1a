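; BP_Key is a coin-shaped key pickup that spins on its yaw axis through a Timeline-driven Lerp.
; When BP_ThirdPersonCharacter overlaps it, the pickup increments that character's TotalKeys, prints a collection message and destroys its coin mesh.
; The actor stays alive through a delay, then spawns a Bp_seedbundle at a hardcoded world location, announces it and destroys itself.
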(event `self.ReceiveBeginPlay`
  (`|ExecutionSequence`
    (:`then_0`
      (bind (_direction _newtrack_1) (`Timeline|Timeline` :!via `SetNewTime` :!label _label)
        (:`Update`
          (`SceneComponent.K2_SetRelativeRotation` (`self.DefaultSceneRoot`) (`KismetMathLibrary.MakeRotator` 0.0 0.0 (`KismetMathLibrary.Lerp` 0.0 360.0 _newtrack_1)) false false))))
    (:`then_1`
      (goto _label))))

(event `self.ReceiveActorBeginOverlap`
  (params (OtherActor :type "Actor Object Reference"))
  (bind _asbp_third_person_character (cast `/Game/ThirdPerson/Blueprints/BP_ThirdPersonCharacter` OtherActor))
  (`/Engine/EditorBlueprintResources/StandardMacros.IncrementInt` (`/Game/ThirdPerson/Blueprints/BP_ThirdPersonCharacter.TotalKeys` _asbp_third_person_character)
    (:`  `
      (`KismetSystemLibrary.PrintText` "Coin Collected!")
      (`ActorComponent.K2_DestroyComponent` (`self.SM_PolygonPrototype_Icon_Coin_01`))
      (`KismetSystemLibrary.Delay` 12.0)
      (`|SpawnActorFromClass` "/Game/blueprints/bp_seedbundle.bp_seedbundle_C" (`KismetMathLibrary.MakeTransform` (-1150.0 -2195.0 610.0)) "Undefined" "MultiplyWithRoot" null null)
      (`KismetSystemLibrary.PrintText` "Seed bundle has spawned!")
      (`self.K2_DestroyActor`))))

(fn `UserConstructionScript`)
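; Cannon actor that launches the third-person character that overlaps it.
; Overlap, or BeginPlay after a short delay, runs LaunchCannonball, which only prints a message, then casts the overlapping actor to BP_ThirdPersonCharacter.
; On a successful cast, it enables physics simulation on the platform and the character's capsule, then adds force to both along the SpawnPoint's forward vector, scaled by Forcee.
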(event `self.ReceiveBeginPlay`
  (`KismetSystemLibrary.Delay` 1.0)
  (`self.Launch cannonball` :!label _label)
  (bind _asbp_third_person_character (cast `/Game/ThirdPerson/Blueprints/BP_ThirdPersonCharacter` (stale `self.ReceiveActorBeginOverlap` OtherActor)))
  (`PrimitiveComponent.SetSimulatePhysics` (`self.platform`) true)
  (`PrimitiveComponent.SetSimulatePhysics` (`Character.CapsuleComponent` _asbp_third_person_character) true)
  (`PrimitiveComponent.AddForce` (`Character.CapsuleComponent` _asbp_third_person_character) (* (`SceneComponent.GetForwardVector` (`self.spawn point`)) (`self.forcee`)) "None" false)
  (`PrimitiveComponent.AddForce` (`self.platform`) (* (`SceneComponent.GetForwardVector` (`self.spawn point`)) (`self.forcee`)) "None" false))

(event `self.ReceiveActorBeginOverlap`
  (params (OtherActor :type "Actor Object Reference"))
  (goto _label))

(event `Launch cannonball`
  (`KismetSystemLibrary.PrintText` "SKY HIGH!!!"))

(fn `UserConstructionScript`)
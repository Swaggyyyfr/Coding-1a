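; Dialogue manager actor that shows lines from a Dialogue array on screen, one per call.
; BeginPlay creates and stores a W_dialouge widget for reuse.
; Each displaynextline call prints the current line, triggers ShowUI to set the widget text and add it to the viewport, then increments Index without a bounds check.
; ShowUI removes the widget after a fixed five-second Delay.
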(event `self.ReceiveBeginPlay`
  (bind _returnvalue (`|CreateWidget` "/Game/blueprints/W_dialouge.W_dialouge_C"))
  (set `self.Widget` _returnvalue))

(event `display next line`
  (`KismetSystemLibrary.PrintText` (`|GetArrayItem` (`self.dialogue`) (`self.index`)))
  (`self.ShowUI`)
  (`/Engine/EditorBlueprintResources/StandardMacros.IncrementInt` (`self.index`)) ; Increment int
)

(event `ShowUI`
  (bind _widget (`self.Widget`))
  (`TextBlock.SetText` (`/Game/blueprints/W_dialouge.TextBlock_9` (`self.Widget`)) (`|GetArrayItem` (`self.dialogue`) (`self.index`)))
  (`UserWidget.AddToViewport` _widget 0) ; Show on screen
  (`KismetSystemLibrary.Delay` 5.0)
  (`Widget.RemoveFromParent` _widget))

(fn `UserConstructionScript`)